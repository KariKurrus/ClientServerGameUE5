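; GS_CountDown is a networked timer, likely a GameState, that counts upward and shows the value on the local player's timer display.
; A looping 0.1-second timer increments TimeCounter on every machine, and the authority copies it to replicated TimeCHacker every tenth count.
; When that differs from the local count, OnRep adopts it and restarts the timer at 1.0 second, unlike the initial rate.
; SetCounter caches the controlled pawn to update its widget.
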(event EventBeginPlay
  (bind _returnvalue (Utilities|Time|SetTimerbyFunctionName 0 "IncreseCount" 0.1 true))
  (Variables|Default|SetTimerHAndler_Counter _returnvalue))

(event EventTick
  (params (DeltaSeconds :type Float%20%28single-precision%29)))

(fn ConstructionScript)

(fn IncreseCount
  (bind _result (Math|Integer|IncrementInt (Variables|Default|GetTimeCounter))
    (:%20%20
      (Networking|SwitchHasAuthority
        (:Authority
          (if (== (Math|Integer|%(Integer) _result 10) 9)
            (Variables|Default|SetTimeCHacker (Variables|Default|GetTimeCounter))
            (CallFunction|SetCounter)
            (else
              (CallFunction|SetCounter))))
        (:Remote
          (CallFunction|SetCounter))))))

(fn OnRepTimeCHacker
  (if (!= (Variables|Default|GetTimeCounter) (Variables|Default|GetTimeCHacker))
    (Variables|Default|SetTimeCounter (Variables|Default|GetTimeCHacker))
    (Utilities|Time|ClearandInvalidateTimerbyHandle (Variables|Default|GetTimerHAndler_Counter))
    (bind _returnvalue (Utilities|Time|SetTimerbyFunctionName 0 "IncreseCount" 1.0 true))
    (Variables|Default|SetTimerHAndler_Counter _returnvalue)
    (CallFunction|SetCounter)))

(fn SetCounter
  (bind _returnvalue (Game|GetPlayerController 0))
  (bind _returnvalue_2 (Pawn|GetControlledPawn _returnvalue))
  (Utilities|IsValid (Variables|Default|GetRef_character)
    (:Is%20Valid
      _)
    (:Is%20Not%20Valid
      (Utilities|IsValid _returnvalue_2
        (:Is%20Valid
          (bind _asbp_player_controller (Utilities|Casting|CastToBP_PlayerController _returnvalue_2))
          (Variables|Default|SetRef_character _asbp_player_controller)))))
  (Utilities|IsValid (Variables|/Game/BluePrints/BP_PlayerController.BP_PlayerController_C|GetRefTimerDisplay (Variables|Default|GetRef_character))
    (:Is%20Valid
      (Default|UpdateTime (Variables|/Game/BluePrints/BP_PlayerController.BP_PlayerController_C|GetRefTimerDisplay (Variables|Default|GetRef_character)) (Variables|Default|GetTimeCounter)))))