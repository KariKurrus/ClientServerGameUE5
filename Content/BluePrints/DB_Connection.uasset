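; Actor that logs level completion stats to a remote PlanetScale SQL database once both player inputs overlap the end zone.
; BeginPlay and Tick test both overlap flags, and a DoOnce opens a single connection using hardcoded credentials.
; On any connection state change, the authority inserts session ID, map name and time counter from the game mode and game state through a string-concatenated query.
; Connection status and query updates print to screen.
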(event Custom|Check
  (Utilities|FlowControl|DoOnce false
    (:Completed
      (Class|MySQLDBConnectionActor|CreateNewConnection "aws.connect.psdb.cloud" "gametwodb" "227hjm5aplk77bhvgxee" "pscale_pw_WGtLck8Gpv2lNmNpJyGu5yMoWW2r6Q2ewbqMt5QACMX" (Utilities|Map|MakeMap "" "")))))

(event EventBeginPlay
  (if (and (Variables|/Game/BluePrints/BP_EnLevelZone.BP_EnLevelZone_C|GetIsOverlapEndZone (Variables|Default|GetFirstInput)) (Variables|/Game/BluePrints/BP_EnLevelZone.BP_EnLevelZone_C|GetIsOverlapEndZone (Variables|Default|GetSecondInput)))
    (Utilities|FlowControl|DoOnce false
      (:Completed
        (Class|MySQLDBConnectionActor|CreateNewConnection "aws.connect.psdb.cloud" "gametwodb" "227hjm5aplk77bhvgxee" "pscale_pw_WGtLck8Gpv2lNmNpJyGu5yMoWW2r6Q2ewbqMt5QACMX" (Utilities|Map|MakeMap "" ""))))))

(event Collision|EventActorBeginOverlap
  (params (OtherActor :type Actor%20Object%20Reference)))

(event EventTick
  (params (DeltaSeconds :type Float%20%28single-precision%29))
  (if (and (Variables|/Game/BluePrints/BP_EnLevelZone.BP_EnLevelZone_C|GetIsOverlapEndZone (Variables|Default|GetFirstInput)) (Variables|/Game/BluePrints/BP_EnLevelZone.BP_EnLevelZone_C|GetIsOverlapEndZone (Variables|Default|GetSecondInput)))
    (CallFunction|Check)))

(event EventOnConnectionStateChanged
  (params (ConnectionStatus :type Boolean) (ConnectionID :type Integer) (ErrorMessage :type String))
  (Variables|Default|SetConnection%20ID ConnectionID)
  (Development|PrintString (Utilities|String|ToString(Boolean) ConnectionStatus))
  (bind _returnvalue (Game|GetCurrentLevelName true))
  (bind _asgsb_count (Utilities|Casting|CastToGSB_Count (Game|GetGameState)))
  (Utilities|IsValid _asgsb_count
    (:Is%20Valid
      (bind _asbp_my_game_mode (Utilities|Casting|CastToBP_MyGameMode (Game|GetGameMode)))
      (Networking|SwitchHasAuthority
        (:Authority
          (Class|MySQLDBConnectionActor|UpdateDatafromQuery (Variables|Default|GetConnection%20ID) (Utilities|String|Append "INSERT INTO DB_GAMETWO_STATS (ID_Session, MAP_Name, PROGRESS_Time) 
VALUES ('" (Utilities|String|ToString(Integer) (Variables|/Game/BluePrints/BP_MyGameMode.BP_MyGameMode_C|GetSession%20ID _asbp_my_game_mode)) "', " "'" _returnvalue "', " (Utilities|String|ToString(Integer) (Variables|/Game/BluePrints/GSB_Count.GSB_Count_C|GetTimeCounter _asgsb_count)) ");")))))))

(event EventOnQueryUpdateStatusChanged
  (params (IsSuccessful :type Boolean) (ErrorMessage :type String))
  (Development|PrintString "succes"))

(fn ConstructionScript)