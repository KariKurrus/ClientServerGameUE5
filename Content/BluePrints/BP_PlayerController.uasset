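; Playable side-scrolling Paper2D character, despite the PlayerController name, that runs along X, jumps, and resets all movable cubes on interact.
; Tick picks the flipbook from alive, falling and speed state, and flips facing by velocity.
; The authority assigns a random name and color, applied to sprite and text through RepNotifies.
; Outside the main menu, it creates a Server/Client status widget, plus a timer widget on possession.
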(event Custom|ADDTImerWidget
  ;[0.1648 1 0.5857] Creating Timer Widget Event
  (bind _returnvalue (Game|GetCurrentLevelName true))
  (if (Utilities|Enum|NotEqual(Enum) _returnvalue "MainMenuLevel")
    (bind _returnvalue_2 (UserInterface|CreateWidget "/Game/UI/WBP_TimerWidget.WBP_TimerWidget_C" (Game|GetPlayerController 0)))
    (bind _output_get (Variables|Default|SetRefTimerDisplay _returnvalue_2))
    (UserInterface|Viewport|AddtoViewport _output_get 0)))

(event Custom|ResolveCubes
  ;[1 0.9157 0.33] Props Reload Logic
  (bind _outactors (Actor|GetAllActorsOfClass "/Game/BluePrints/BP_MovableCubeSM.BP_MovableCubeSM_C"))
  (for _array_element _outactors
    (Default|SettoDefaultPosition _array_element)
    (Development|PrintString "Props Reset!")))

(event Custom|CreteUI
  (params (InText :type Text) (InColorAndOpacity :type Slate%20Color%20Structure))
  ;[0.3551 1 0.9382] Creating User UI logic
  (bind _returnvalue (UserInterface|CreateWidget "/Game/UI/WBP_HostOnlyUI.WBP_HostOnlyUI_C" (Game|GetPlayerController 0)))
  (Variables|Default|SetUIid _returnvalue)
  (UserInterface|Viewport|AddtoViewport _returnvalue 0)
  (Default|SetConnectionType _returnvalue InText InColorAndOpacity)
  (bind _outactors (Actor|GetAllActorsOfClass "BP_PlayerController_C"))
  (for (_array_element _array_index) _outactors
    (if (== _array_index 0)
      (Default|SetColorandName (Variables|Default|GetUIid) (Math|Conversions|ToLinearColor(Color) (Variables|BP_PlayerController_C|GetColorPreset _array_element)) (Variables|BP_PlayerController_C|GetCurrentName _array_element)))))

(event EventBeginPlay
  ;[0.1421 0.1563 1] On Creating Object Event
  ;;[1 1 1] Setting Character
  (CallFunction|SetRandomNameNcolor)
  ;;[1 1 1] UI SpawnCheck
  (bind _returnvalue (Game|GetCurrentLevelName true))
  ;;[1 1 1] UI Creating
  (if (Utilities|Enum|NotEqual(Enum) _returnvalue "MainMenuLevel")
    (Networking|SwitchHasAuthority
      (:Authority
        (CallFunction|CreteUI "Server" (Utilities|Struct|MakeSlateColor "(R=0.000000,G=1.000000,B=0.164729,A=1.000000)" "UseColor_Specified")))
      (:Remote
        (CallFunction|CreteUI "Client" (Utilities|Struct|MakeSlateColor "(R=0.178210,G=0.081099,B=1.000000,A=1.000000)" "UseColor_Specified"))))))

(event EventPossessed
  (params (NewController :type Controller%20Object%20Reference))
  ;[0.5006 0.1127 1] Adding Timer Widget
  (CallFunction|ADDTImerWidget))

(event EventTick
  (params (DeltaSeconds :type Float%20%28single-precision%29))
  ;[1 0.1976 0.1916] Updating Events
  (CallFunction|UpdateAnimation)
  (CallFunction|UpdateRotation))

(event Input|ActionEvents|InputActionJump
  (params (Key :type Key%20Structure :default "None"))
  ;[1 0.2579 0.09172] Jumping
  (:Pressed
    (Character|Jump))
  (:Released
    (Character|StopJumping)))

(event Input|ActionEvents|InputActionInteractAction
  (params (Key :type Key%20Structure :default "None"))
  ;[1 0.1264 0.5435] Use 'E' button to reload props
  (:Pressed
    (Variables|Default|SetIsResolvingCubes true)
    (CallFunction|ResolveCubes)
    (Utilities|FlowControl|Delay 0.1)
    (Variables|Default|SetIsResolvingCubes false)))

(event Input|AxisEvents|InputAxisMove
  (params (AxisValue :type Float%20%28single-precision%29))
  ;[0.235 1 0.1782] Movement
  (bind _output_get (Variables|Default|SetAxis%20Value AxisValue))
  (Pawn|Input|AddMovementInput "1.000000, 0, 0" _output_get false))

(fn ConstructionScript)

(fn UpdateAnimation
  (Sprite|SetFlipbook (Variables|Default|GetSprite) (select (not (Variables|Default|GetisAlive)) "/Game/Animations/Die/FB_Died.FB_Died" (select (AI|Components|NavMovement|IsFalling (Variables|Character|GetCharacterMovement)) "/Game/Animations/Jump/FB_Jump.FB_Jump" (select (> (Math|Vector|VectorLength (Variables|/Script/Engine.MovementComponent|GetVelocity (Variables|Character|GetCharacterMovement))) 0.0) "/Game/Animations/Run/FB_Run.FB_Run" "/Game/Animations/Idle/FB_Idle.FB_Idle")))))

(fn UpdateRotation
  (Math|Float|CompareFloat (.X (Math|Vector|BreakVector (Variables|/Script/Engine.MovementComponent|GetVelocity (Variables|Character|GetCharacterMovement)))) 0.0
    (:>
      (Transformation|SetActorRotation (Math|Rotator|MakeRotator 0.0 0.0 0.0)))
    (:<
      (Transformation|SetActorRotation (Math|Rotator|MakeRotator 0.0 0.0 1.8e+02)))))

(fn SetRandomNameNcolor
  (Networking|SwitchHasAuthority
    (:Authority
      (Variables|Default|SetColorPreset (Math|Color|MakeColor (Math|Conversions|ToByte(Integer) (Math|Random|RandomIntegerinRange 0 255)) (Math|Conversions|ToByte(Integer) (Math|Random|RandomIntegerinRange 0 255)) (Math|Conversions|ToByte(Integer) (Math|Random|RandomIntegerinRange 0 255)) 225))
      (Variables|Default|SetCurrentName (Utilities|Text|ToText(String) (.OutItem (Utilities|Array|Random (Utilities|String|ParseIntoArray (Variables|Default|GetNameList) "."))))))))

(fn OnRepColorPreset
  (bind _colorpreset (Variables|Default|GetColorPreset))
  (Rendering|Components|TextRender|SetTextRenderColor (Variables|Default|GetTextRender) (Variables|Default|GetColorPreset))
  (Sprite|SetSpriteColor (Variables|Default|GetSprite) (Math|Conversions|ToLinearColor(Color) (Math|Color|MakeColor (.b _colorpreset) (.g _colorpreset) (.r _colorpreset) (.a _colorpreset)))))

(fn OnRepCurrntName
  (Rendering|Components|TextRender|SetText (Variables|Default|GetTextRender) (Variables|Default|GetCurrentName)))

(fn NewFunction0)

(event Input|ActionEvents|InputActionJump
  (params (Key :type Key%20Structure :default "None")))