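; BP_PoisionPlace is a trigger volume that teleports any overlapping BP_PlayerController actor to a reference point, with no damage logic of its own.
; On overlap it confirms the actor against all BP_PlayerController instances, stores it, then teleports it slightly above TeleportReference1.
; TeleportReference2 serves as the fallback if that teleport fails; both destinations take only X and Z from the reference.
; The construction script scales the Box from SizeParam.
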(event EventBeginPlay)

(event Collision|EventActorBeginOverlap
  (params (OtherActor :type Actor%20Object%20Reference))
  (bind _teleportreference1 (Variables|Default|GetTeleportReference1))
  (bind _teleportreference2 (Variables|Default|GetTeleportReference2))
  (bind _tr (Variables|/Game/BluePrints/BP_TpZone.BP_TpZone_C|Gettr _teleportreference1))
  (bind _tr_2 (Variables|/Game/BluePrints/BP_TpZone.BP_TpZone_C|Gettr _teleportreference2))
  (bind _returnvalue (Transformation|GetWorldLocation _tr))
  (bind _returnvalue_2 (Transformation|GetWorldLocation _tr_2))
  (Variables|Default|SetCurrentActorOverlap OtherActor)
  (bind _outactors (Actor|GetAllActorsOfClass "/Game/BluePrints/BP_PlayerController.BP_PlayerController_C"))
  (for _array_element _outactors
    (if (== _array_element (Variables|Default|GetCurrentActorOverlap))
      (bind _asbp_player_controller (Utilities|Casting|CastToBP_PlayerController (Variables|Default|GetCurrentActorOverlap)))
      (Variables|Default|SetCurrentBp_PlayerControllerOverlap _asbp_player_controller)
      (bind _returnvalue_3 (Transformation|Teleport (Variables|Default|GetCurrentActorOverlap) (Math|Vector|MakeVector (.x _returnvalue) 0.0 (+ (.z _returnvalue) 1e+01)) "0, 0, 0"))
      (if (not _returnvalue_3)
        (Transformation|Teleport (Variables|Default|GetCurrentActorOverlap) (Math|Vector|MakeVector (.x _returnvalue_2) 0.0 (+ (.z _returnvalue_2) 1e+01)) "0, 0, 0")))))

(event EventTick
  (params (DeltaSeconds :type Float%20%28single-precision%29)))

(fn ConstructionScript
  (Transformation|SetWorldScale3D (Variables|Default|GetBox) (Variables|Default|GetSizeParam)))