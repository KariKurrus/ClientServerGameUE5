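; GSB_Count keeps a running seconds counter that stays in sync between server and clients and feeds an on-screen timer.
; Each machine increments TimeCounter on a looping one-second timer and updates the local player pawn's RefTimerDisplay, caching that pawn reference.
; To avoid replicating every tick, the authority copies the count into TimeChecker every ten seconds.
; Its OnRep corrects any drift on clients and restarts their local timer.
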(event EventBeginPlay
  (bind _returnvalue (Utilities|Time|SetTimerbyFunctionName 0 "IncreaseCount" 1.0 true))
  (Variables|Default|SetTimeHandlerCounter _returnvalue))

(fn ConstructionScript)

(fn IncreaseCount
  (bind _result (Math|Integer|IncrementInt (Variables|Default|GetTimeCounter))
    (:%20%20
      (Networking|SwitchHasAuthority
        (:Authority
          (if (== (Math|Integer|%(Integer) _result 10) 1)
            (Variables|Default|SetTimeChecker (Variables|Default|GetTimeCounter))
            (CallFunction|SetCounter)
            (else
              (CallFunction|SetCounter))))
        (:Remote
          (CallFunction|SetCounter))))))

(fn SetCounter
  (bind _returnvalue (Game|GetPlayerController 0))
  (bind _returnvalue_2 (Pawn|GetControlledPawn _returnvalue))
  (Utilities|IsValid (Variables|Default|GetRef%20Character)
    (:Is%20Valid
      _)
    (:Is%20Not%20Valid
      (Utilities|IsValid _returnvalue_2
        (:Is%20Valid
          (bind _asbp_player_controller (Utilities|Casting|CastToBP_PlayerController _returnvalue_2))
          (Variables|Default|SetRef%20Character _asbp_player_controller)))))
  (Utilities|IsValid (Variables|/Game/BluePrints/BP_PlayerController.BP_PlayerController_C|GetRefTimerDisplay (Variables|Default|GetRef%20Character))
    (:Is%20Valid
      (Default|UpdateTime (Variables|/Game/BluePrints/BP_PlayerController.BP_PlayerController_C|GetRefTimerDisplay (Variables|Default|GetRef%20Character)) (Variables|Default|GetTimeCounter)))))

(fn OnRepTimeChecker
  (if (!= (Variables|Default|GetTimeCounter) (Variables|Default|GetTimeChecker))
    (Variables|Default|SetTimeCounter (Variables|Default|GetTimeChecker))
    (Utilities|Time|ClearandInvalidateTimerbyHandle (Variables|Default|GetTimeHandlerCounter))
    (bind _returnvalue (Utilities|Time|SetTimerbyFunctionName 0 "IncreaseCount" 1.0 true))
    (Variables|Default|SetTimeHandlerCounter _returnvalue)
    (CallFunction|SetCounter)))