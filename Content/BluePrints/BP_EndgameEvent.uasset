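; BP_EndgameEvent is an end-of-level trigger that moves the game to a new map when both end-zone conditions are met.
; Each tick it checks the end-zone overlap flags on two referenced inputs, FirstInput and SecondInput.
; When both are set, it reveals a text render, waits through a short delay, then calls ServerTravel on BP_MyGameMode to load NewMap.
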(event EventBeginPlay)

(event Collision|EventActorBeginOverlap
  (params (OtherActor :type Actor%20Object%20Reference)))

(event EventTick
  (params (DeltaSeconds :type Float%20%28single-precision%29))
  (if (and (Variables|/Game/BluePrints/BP_EnLevelZone.BP_EnLevelZone_C|GetIsOverlapEndZone (Variables|Default|GetSecondInput)) (Variables|/Game/BluePrints/BP_EnLevelZone.BP_EnLevelZone_C|GetIsOverlapEndZone (Variables|Default|GetFirstInput)))
    (Rendering|SetVisibility (Variables|Default|GetTextRender) true false)
    (Utilities|FlowControl|Delay 5.0)
    (bind _asbp_my_game_mode (Utilities|Casting|CastToBP_MyGameMode (Game|GetGameMode)))
    (Default|ServerTravel _asbp_my_game_mode "NewMap")))

(fn ConstructionScript)