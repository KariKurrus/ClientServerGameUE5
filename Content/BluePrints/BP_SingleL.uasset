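; BP_SingleL is a lever-like toggle actor whose Stick swings between two opposite tilts when triggered by overlap.
; When anything begins overlapping the Box, it loops over all BP_PlayerController actors and checks whether each overlaps the Box.
; A match flips IsTriggered and animates the Stick to the other angle over one second with MoveComponentTo.
; Non-matching actors only print a debug message.
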(event OnComponentBeginOverlap(Box)
  (params (OverlappedComponent :type Primitive%20Component%20Object%20Reference) (OtherActor :type Actor%20Object%20Reference) (OtherComp :type Primitive%20Component%20Object%20Reference) (OtherBodyIndex :type Integer) (bFromSweep :type Boolean) (SweepResult :type Hit%20Result%20Structure%20%28by%20ref%29))
  (bind _outactors (Actor|GetAllActorsOfClass "/Game/BluePrints/BP_PlayerController.BP_PlayerController_C"))
  (for _array_element _outactors
    (if (Collision|IsOverlappingActor (Variables|Default|GetBox) _array_element :!class /Script/Engine.PrimitiveComponent)
      (if (not (Variables|Default|GetIsTriggered))
        (Components|MoveComponentTo (Variables|Default|GetStick) "0.000000,0.000000,100.000000" "-40.000000,0.000000,0.000000" false false 1.0 false)
        (Variables|Default|SetIsTriggered true)
        (else
          (Components|MoveComponentTo (Variables|Default|GetStick) "0.000000,0.000000,100.000000" "40.000000,0.000000,0.000000" false false 1.0 false)
          (Variables|Default|SetIsTriggered false)))
      (else
        (Development|PrintString "Hello")))))

(event EventBeginPlay)

(event Collision|EventActorBeginOverlap
  (params (OtherActor :type Actor%20Object%20Reference)))

(event EventTick
  (params (DeltaSeconds :type Float%20%28single-precision%29)))

(fn ConstructionScript)