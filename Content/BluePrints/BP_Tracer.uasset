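; BP_Tracer is a sensor actor that drives a linked door based on whether something is in front of it.
; Every tick it runs a short forward line trace for physics bodies and pawns, drawing a debug line.
; A hit passes MoveToPin to MoveBlock on the ControlDoor reference, while a miss passes zero.
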(event EventBeginPlay)

(event EventTick
  (params (DeltaSeconds :type Float%20%28single-precision%29))
  (bind _controldoor (Variables|Default|GetControlDoor))
  (bind _returnvalue (Collision|LineTraceForObjects (Transformation|GetActorLocation) (+ (Transformation|GetActorLocation) (* (Math|Vector|GetForwardVector (Transformation|GetActorRotation)) 2e+02)) (Utilities|Array|MakeArray "ObjectTypeQuery4" "ObjectTypeQuery3") false 0 "ForOneFrame" true "(R=1.000000,G=0.000000,B=0.000000,A=1.000000)" "(R=1.000000,G=0.004391,B=0.000000,A=1.000000)" 0.0))
  (if _returnvalue
    (Default|MoveBlock _controldoor (Variables|Default|GetMoveToPin))
    (else
      (Default|MoveBlock _controldoor 0.0))))

(fn ConstructionScript)