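; BP_MyGameMode is a game mode that handles level travel and runs a rudimentary automated test of player names.
; The ServerTravel event runs the servertravel console command with the given level name.
; On the first Tick, a DoOnce calls AutoTestCore, whose PlayerTest prints expected and real names for every BP_PlayerController.
; Both values read CurrentName, so the comparison checks the name against itself.
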(event Custom|ServerTravel
  (params (Level%20name :type String))
  (Development|ExecuteConsoleCommand (Utilities|String|Append "servertravel " Level%20name) 0))

(event EventBeginPlay)

(event EventTick
  (params (DeltaSeconds :type Float%20%28single-precision%29))
  (Utilities|FlowControl|DoOnce false
    (:Completed
      (CallFunction|AutoTestCore))))

(fn ConstructionScript)

(fn AutoTestCore
  (CallFunction|PlayerTest))

(fn PlayerTest
  (bind _outactors (Actor|GetAllActorsOfClass "/Game/BluePrints/BP_PlayerController.BP_PlayerController_C"))
  (for _array_element _outactors
    (Development|PrintString (Utilities|String|Append "Expected:   " (Utilities|String|Append (Utilities|String|ToString(Text) (Variables|/Game/BluePrints/BP_PlayerController.BP_PlayerController_C|GetCurrentName _array_element)) (Utilities|String|Append "  ||||  Real:   " (Utilities|String|Append (Utilities|String|ToString(Text) (Variables|/Game/BluePrints/BP_PlayerController.BP_PlayerController_C|GetCurrentName _array_element)) (Utilities|String|Append "Result:   " (Utilities|String|ToString(Boolean) (Utilities|Enum|Equal(Enum) (Utilities|String|ToString(Text) (Variables|/Game/BluePrints/BP_PlayerController.BP_PlayerController_C|GetCurrentName _array_element)) (Utilities|String|ToString(Text) (Variables|/Game/BluePrints/BP_PlayerController.BP_PlayerController_C|GetCurrentName _array_element))))))))) true true "(R=1.000000,G=0.797874,B=0.028262,A=1.000000)" 1e+01)))