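; BP_DoorByL is a door Blueprint that raises and lowers its static mesh according to a single input's triggered state.
; The construction script caches the mesh's world location as StartPosition.
; Every Tick checks OneInput.IsTriggered and calls MoveComponentTo toward StartPosition raised by WayLenVar on Z, or back to StartPosition.
; That cached world position is passed as a relative-location target.
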(event EventBeginPlay)

(event Collision|EventActorBeginOverlap
  (params (OtherActor :type Actor%20Object%20Reference)))

(event EventTick
  (params (DeltaSeconds :type Float%20%28single-precision%29))
  (bind _startposition (Variables|Default|GetStartPosition))
  (bind _startposition_2 (Variables|Default|GetStartPosition))
  (if (Variables|/Game/BluePrints/BP_SingleL.BP_SingleL_C|GetIsTriggered (Variables|Default|GetOneInput))
    (Components|MoveComponentTo (Variables|Debug|GetStaticMeshComponent) (Math|Vector|MakeVector (.x _startposition_2) (.y _startposition_2) (+ (.z _startposition_2) (Variables|Default|GetWayLenVar))) "0, 0, 0" false false 0.2 false)
    (else
      (Components|MoveComponentTo (Variables|Debug|GetStaticMeshComponent) (Math|Vector|MakeVector (.x _startposition) (.y _startposition) (+ (.z _startposition) 0.0)) "0, 0, 0" false false 0.2 false))))

(fn ConstructionScript
  (Variables|Default|SetStartPosition (Transformation|GetWorldLocation (Variables|Debug|GetStaticMeshComponent))))